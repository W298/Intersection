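; A spline actor Blueprint that exposes attachment points at both ends of its spline.
; The construction script gathers the child components of the StartPoints and EndPoints components into a ConnectionPoints array.
; It then moves each group to the first or last spline point, facing along that point's tangent.
; GetSplineAttachmentPoints returns the array, and the event graph holds only disabled default events.
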(event EventBeginPlay
  (|CallParentFunction) ; This node is disabled and will not be called.\nDrag off pins to build functionality.
)

(event Collision|EventActorBeginOverlap
  (params (OtherActor :type Actor%20Object%20Reference))
  (|CallParentFunction OtherActor) ; This node is disabled and will not be called.\nDrag off pins to build functionality.
)

(event EventTick
  (params (DeltaSeconds :type Float%20%28single-precision%29))
  (|CallParentFunction DeltaSeconds) ; This node is disabled and will not be called.\nDrag off pins to build functionality.
)

(fn ConstructionScript
  (bind _connectionpoints (Variables|Default|GetConnectionPoints))
  (bind _spline (Variables|Default|GetSpline))
  (bind (_location _tangent) (Spline|GetLocationandTangentatSplinePoint _spline 0 "World"))
  (bind _returnvalue (Spline|GetNumberOfSplinePoints _spline))
  (bind _returnvalue_2 (- _returnvalue 1))
  (bind (_location_2 _tangent_2) (Spline|GetLocationandTangentatSplinePoint _spline _returnvalue_2 "World"))
  (|CallParentFunction)
  (Utilities|FlowControl|Sequence
    (:then_0
      (Utilities|Array|Clear _connectionpoints)
      (Utilities|Array|AppendArray _connectionpoints (Components|GetChildrenComponents (Variables|Default|GetStartPoints) false))
      (Utilities|Array|AppendArray _connectionpoints (Components|GetChildrenComponents (Variables|Default|GetEndPoints) false)))
    (:then_1
      (Transformation|SetWorldLocationAndRotation (Variables|Default|GetStartPoints) _location (Math|Conversions|RotationFromXVector _tangent) false false))
    (:then_2
      (Transformation|SetWorldLocationAndRotation (Variables|Default|GetEndPoints) _location_2 (Math|Conversions|RotationFromXVector _tangent_2) false false))))

(fn GetSplineAttachmentPoints
  (return (Variables|Default|GetConnectionPoints)))